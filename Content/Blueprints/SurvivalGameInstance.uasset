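; Survival game instance that manages the game's UI: runtime UI, message box, pickup panel and inventory, plus message pushing.
; ShowPanel lazily creates each widget into a by-ref variable, avoids duplicates, increments an active count and enables Game-and-UI input with cursor.
; HidePanel removes a panel, restoring game-only input and hiding the cursor when the count reaches zero.
; The message box also uses ShowPanel, so it counts as active.
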(event `Show RunTime UI`
  ;[1 1 1] 创建运行时间UI
  (`|ExecutionSequence`
    (:`then_0`
      (`/Engine/EditorBlueprintResources/StandardMacros.IsValid` (`self.RunTimeUI`)
        (:`Is Not Valid`
          (bind _returnvalue (`|CreateWidget` "/Game/UI/UI_RunTimeUI.UI_RunTimeUI_C" (`GameplayStatics.GetPlayerController` 0)))
          (bind _output_get (set `self.RunTimeUI` _returnvalue))
          (`UserWidget.AddToViewport` _output_get 0))))
    (:`then_1`
      ;[1 1 1] 消息提醒
      (`self.ShowPanel` "/Game/UI/UI_MessageBox.UI_MessageBox_C" (`self.Message Box`)))))

(event `ShowPickablePanel`
  ;[1 1 1] 创建拾取UI
  (`self.ShowPanel` "/Game/UI/UI_PickablePanel.UI_PickablePanel_C" (`self.PickablePanel`)))

(event `HidePickablePanel`
  ;[1 1 1] 隐藏拾取UI(当列表内无物品时)
  (`self.HidePanel` (`self.PickablePanel`)))

(event `Show Inventory Panel`
  ;[1 1 1] 显示背包页面UI
  (`self.ShowPanel` "/Game/UI/UI_Inventory.UI_Inventory_C" (`self.Inventory Panel`)))

(event `Hide Inventory Panel`
  ;[1 1 1] 隐藏背包界面
  (`self.HidePanel` (`self.Inventory Panel`)))

(event `Push Message`
  (params (TextContent :type String))
  ;[1 1 1] 消息提醒
  (`/Game/UI/UI_MessageBox.Push Message` (`self.Message Box`) TextContent))

(fn `HidePanel`
  (params (PanelVar :type "Widget Object Reference"))
  (bind _returnvalue (`GameplayStatics.GetPlayerController` 0))
  ;[1 1 1] 隐藏拾取UI(当列表内无物品时)
  (`/Engine/EditorBlueprintResources/StandardMacros.IsValid` PanelVar
    (:`Is Valid`
      (`Widget.RemoveFromParent` PanelVar)
      (bind _result (`/Engine/EditorBlueprintResources/StandardMacros.DecrementInt` (`self.ActiveUICount`))
        (:`  `
          (if (== _result 0)
            ;[1 1 1] 设置输入方式（GAME）
            (`WidgetBlueprintLibrary.SetInputMode_GameOnly` _returnvalue)
            (set `PlayerController.bShowMouseCursor` false _returnvalue)))))))

(fn `ShowPanel`
  (params (`Panel Type Clas` :type "UserWidget Class Reference") (PanelVariable :type "UserWidget Object Reference (by ref)"))
  (bind _returnvalue (`GameplayStatics.GetPlayerController` 0))
  ;[1 1 1] 防止重复产生UI
  (`/Engine/EditorBlueprintResources/StandardMacros.IsValid` PanelVariable
    (:`Is Valid`
      ;[1 1 1] 判断拾取UI是否已经可见
      (if (not (`Widget.IsInViewport` PanelVariable))
        (`UserWidget.AddToViewport` PanelVariable 0 :!label _label)
        (`/Engine/EditorBlueprintResources/StandardMacros.IncrementInt` (`self.ActiveUICount`)
          (:`  `
            (`WidgetBlueprintLibrary.SetInputMode_GameAndUIEx` _returnvalue PanelVariable)
            (set `PlayerController.bShowMouseCursor` true _returnvalue)))))
    (:`Is Not Valid`
      (bind _returnvalue_2 (`|CreateWidget` `Panel Type Clas` (`GameplayStatics.GetPlayerController` 0)))
      (`|VariableSetRef` PanelVariable _returnvalue_2)
      (goto _label))))