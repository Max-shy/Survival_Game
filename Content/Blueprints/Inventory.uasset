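; Inventory Blueprint that adds item slots to a backpack under a weight-based capacity limit.
; TestCaopacity reads the item type's Weight from class defaults, multiplies it by Count and checks the resulting Load against Capacity.
; On success, TryAddItem updates Load, then either increments the count on a Content slot of the same type or appends a new one, returning whether the item fit.
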(fn `TestCaopacity`
  (params (`New Item` :type "/Game/Blueprints/ItemSlot Structure"))
  (returns (Success :type Boolean) (`New Load` :type Integer))
  (bind (_type _name _icon _count) (break `/Game/Blueprints/ItemSlot` `New Item`))
  (bind _returnvalue (+ (* (`.Weight` (defaults `Object` _type)) _count) (`self.Load`)))
  ;[1 1 1] 测试背包容量
  (return (and (<= (`self.Load`) (`self.Capacity`)) (<= _returnvalue (`self.Capacity`))) _returnvalue))

(fn `TryAddItem`
  (params (NewItem :type "/Game/Blueprints/ItemSlot Structure"))
  (returns (Success :type Boolean))
  (bind (_type _name _icon _count) (break `/Game/Blueprints/ItemSlot` NewItem))
  ;[1 1 1] 背包添加Item功能
  (bind (_success _new_load) (`self.TestCaopacity` NewItem))
  (if _success
    (set `self.Load` _new_load)
    (for _array_element (`self.Content`)
      (bind (_type_2 _name_2 _icon_2 _count_2) (break `/Game/Blueprints/ItemSlot` _array_element))
      (if (== _type_2 _type)
        (setmembers `/Game/Blueprints/ItemSlot` :`StructRef` _array_element :`Type` _type_2 :`Name` _name_2 :`Icon` _icon_2 :`Count` (+ _count_2 _count))
        (return true)))
    (`KismetArrayLibrary.Array_Add` (`self.Content`) NewItem)
    (return true)
    (else
      (return false))))