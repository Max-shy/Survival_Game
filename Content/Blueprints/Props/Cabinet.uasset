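; Storage cabinet prop that holds a list of item slots and shows its UI panel while the survival character is nearby.
; Overlaps on AffectArea tell the SurvivalGameInstance to show or hide the cabinet panel.
; AddItem stacks by item type or appends a new slot, while RemoveItem decrements the count or removes the emptied slot.
; Dispatchers broadcast added, removed and count-updated changes.
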(event `self.Affect Area.OnComponentBeginOverlap`
  (params (OverlappedComponent :type "PrimitiveComponent Object Reference") (OtherActor :type "Actor Object Reference") (OtherComp :type "PrimitiveComponent Object Reference") (OtherBodyIndex :type Integer) (bFromSweep :type Boolean) (SweepResult :type "HitResult Structure (by ref)"))
  (cast `/Game/Blueprints/SurvivalCharacter` OtherActor)
  (`/Game/Blueprints/SurvivalGameInstance.Show Cabinet Panel` (cast `/Game/Blueprints/SurvivalGameInstance` (`GameplayStatics.GetGameInstance`) :!pure true)))

(event `self.Affect Area.OnComponentEndOverlap`
  (params (OverlappedComponent :type "PrimitiveComponent Object Reference") (OtherActor :type "Actor Object Reference") (OtherComp :type "PrimitiveComponent Object Reference") (OtherBodyIndex :type Integer))
  (cast `/Game/Blueprints/SurvivalCharacter` OtherActor)
  (`/Game/Blueprints/SurvivalGameInstance.Hide Cabinet Panel` (cast `/Game/Blueprints/SurvivalGameInstance` (`GameplayStatics.GetGameInstance`) :!pure true)))

(fn `AddItem`
  (params (NewItem :type "/Game/Blueprints/ItemSlot Structure"))
  (for (_array_element _array_index) (`self.Content`)
    (bind (_type _name _icon _count) (break `/Game/Blueprints/ItemSlot` _array_element))
    (if (== (`.Type_12_D07D63624DB3F0CCC74B0590BA5DFFFE` (break `/Game/Blueprints/ItemSlot` NewItem)) _type)
      ;[1 1 1] 存储箱中有New Item
      (bind _structout (setmembers `/Game/Blueprints/ItemSlot` :`StructRef` (`|GetArrayItem` (`self.Content`) _array_index) :`Count` (+ _count 1)))
      (`self.UpdatedItemCount` _structout)
      (return)))
  ;[1 1 1] 存储箱中无New Item
  (`KismetArrayLibrary.Array_Add` (`self.Content`) NewItem)
  (`self.AddedItem` (struct))
  (return))

(fn `RemoveItem`
  (params (RemovedItem :type "/Game/Blueprints/ItemSlot Structure"))
  (for (_array_element _array_index) (`self.Content`)
    (bind (_type _name _icon _count) (break `/Game/Blueprints/ItemSlot` _array_element))
    (if (== (`.Type_12_D07D63624DB3F0CCC74B0590BA5DFFFE` (break `/Game/Blueprints/ItemSlot` RemovedItem)) _type)
      (bind _returnvalue (- _count 1))
      (if (> _returnvalue 0)
        (bind _structout (setmembers `/Game/Blueprints/ItemSlot` :`StructRef` (`|GetArrayItem` (`self.Content`) _array_index) :`Count` _returnvalue))
        (`self.UpdatedItemCount` _structout)
        (else
          (`KismetArrayLibrary.Array_RemoveItem` (`self.Content`))
          (`self.RemovedItem` RemovedItem)))
      (return))))

(fn `UserConstructionScript`)