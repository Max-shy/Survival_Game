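; GlobalTimer is an actor that runs a game-wide clock and day-night cycle from game time, offset a quarter day to start at dawn.
; Each tick it rotates the sun light to match the time, updates the sky sphere and recaptures the sky light.
; It also refreshes day, hour and minute, printing a message when crossing the 6:00 or 18:00 boundary.
; The EnterDayTime and EnterNightTime events are empty stubs.
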(event `self.ReceiveTick`
  (params (DeltaSeconds :type "Float (single-precision)"))
  (bind _secondsperday (`self.SecondsPerDay`))
  (bind _secondsperday_2 (`self.SecondsPerDay`))
  (bind _returnvalue (/ _secondsperday 24.0))
  (bind (_remainder _returnvalue_2) (`KismetMathLibrary.FMod` (+ (`KismetSystemLibrary.GetGameTimeInSeconds`) (/ _secondsperday 4.0)) _secondsperday))
  (bind (_remainder_2 _returnvalue_3) (`KismetMathLibrary.FMod` _remainder _returnvalue))
  (`self.K2_SetActorRotation` (`self.SunLight`) (`KismetMathLibrary.MakeRotator` 0.0 (+ (* -360 (/ (`KismetMathLibrary.FMod` (+ (`KismetSystemLibrary.GetGameTimeInSeconds`) (/ _secondsperday_2 4.0)) _secondsperday_2) _secondsperday_2)) 90.0)) false)
  (`/Engine/EngineSky/BP_Sky_Sphere.UpdateSunDirection` (`self.SkySphere`))
  (`SkyLightComponent.RecaptureSky` (`SkyLight.LightComponent` (`self.SkyLight`)))
  (`|ExecutionSequence`
    (:`then_0`
      (set `self.CurrentDay` (+ _returnvalue_2 1)))
    (:`then_1`
      (bind _output_get (set `self.CurrentHour` _returnvalue_3))
      ;[1 1 1] 当前帧昼夜状态
      ;;[1 1 1] 先判断转换，再更新状态
      (`|ExecutionSequence`
        (:`then_0`
          (bind _returnvalue_4 (and (>= _output_get 6) (< _output_get 18)))
          (if _returnvalue_4
            ;[1 1 1] 夜->昼状态转换
            (if (not (`self.IsDayTime`))
              (`KismetSystemLibrary.PrintString` "天亮了！"))
            (else
              ;[1 1 1] 昼->夜状态转换
              (if (`self.IsDayTime`)
                (`KismetSystemLibrary.PrintString` "天黑了！")))))
        (:`then_1`
          (set `self.IsDayTime` _returnvalue_4))))
    (:`then_2`
      (set `self.CurrentMinute` (`.ReturnValue` (`KismetMathLibrary.FMod` _remainder_2 (/ _returnvalue 60.0)))))))

(event `Enter Day Time`)

(event `Enter Night Time`)

(fn `UserConstructionScript`)